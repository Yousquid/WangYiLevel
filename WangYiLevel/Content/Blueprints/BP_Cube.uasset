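; Interactable cube actor that attaches to the third-person character while the player interacts with it.
; BeginPlay caches the character, and the Fwd component's overlap events toggle that character's CanInteractBox flag for any overlapping object, without filtering.
; Tick polls the character's flags, re-attaching the cube every frame while IsinteractingBox and CanInteractBox are both true and detaching it otherwise, with KeepRelative rules for both.
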(event `self.ReceiveBeginPlay`
  (bind _returnvalue (`GameplayStatics.GetActorOfClass` "/Game/ThirdPerson/Blueprints/BP_ThirdPersonCharacter.BP_ThirdPersonCharacter_C"))
  (set `self.CharacterReference` _returnvalue))

(event `self.Fwd.OnComponentBeginOverlap`
  (params (OverlappedComponent :type "PrimitiveComponent Object Reference") (OtherActor :type "Actor Object Reference") (OtherComp :type "PrimitiveComponent Object Reference") (OtherBodyIndex :type Integer) (bFromSweep :type Boolean) (SweepResult :type "HitResult Structure (by ref)"))
  (set `/Game/ThirdPerson/Blueprints/BP_ThirdPersonCharacter.CanInteractBox` true (`self.CharacterReference`)))

(event `self.Fwd.OnComponentEndOverlap`
  (params (OverlappedComponent :type "PrimitiveComponent Object Reference") (OtherActor :type "Actor Object Reference") (OtherComp :type "PrimitiveComponent Object Reference") (OtherBodyIndex :type Integer))
  (set `/Game/ThirdPerson/Blueprints/BP_ThirdPersonCharacter.CanInteractBox` false (`self.CharacterReference`)))

(event `self.ReceiveTick`
  (params (DeltaSeconds :type "Float (single-precision)"))
  (bind _characterreference (`self.CharacterReference`))
  (if (`/Game/ThirdPerson/Blueprints/BP_ThirdPersonCharacter.IsinteractingBox` _characterreference)
    (if (`/Game/ThirdPerson/Blueprints/BP_ThirdPersonCharacter.CanInteractBox` _characterreference)
      (`self.K2_AttachToActor` _characterreference "None" "KeepRelative" "KeepRelative" "KeepRelative")
      (else
        (`self.K2_DetachFromActor` "KeepRelative")))
    (else
      (`self.K2_DetachFromActor` "KeepRelative"))))

(fn `UserConstructionScript`)