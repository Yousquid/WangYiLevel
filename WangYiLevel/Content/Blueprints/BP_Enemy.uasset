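; Enemy AI that patrols two waypoints, or idles when none are set, and chases the player once alerted.
; Perception updates from the third-person character toggle a sight flag, with sight loss restoring walk speed and restarting patrol.
; Tick raises or lowers Alertness from that flag and feeds a camera-facing alert bar widget.
; Full alertness issues a move-to on the target, with a DoOnce gating the switch to running.
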(event `self.ReceiveBeginPlay`
  (`self.Patrol`)
  (set `self.Alertness` 0.0))

(event `Patrol`
  (set `CharacterMovementComponent.MaxWalkSpeed` 150.0 (`self.CharacterMovement`))
  (if (> (`KismetArrayLibrary.Array_Length` (`self.PatrolLocation`)) 0)
    (`|AIMoveTo` self (`|GetArrayItem` (`self.PatrolLocation`) (`self.Locations`)) null
      (:`OnSuccess`
        (`KismetSystemLibrary.Delay` (`KismetMathLibrary.RandomFloatInRange` 0.5 1.2))
        (`self.Patrol`)
        (`/Engine/EditorBlueprintResources/StandardMacros.IncrementInt` (`self.Locations`)
          (:`  `
            (if (== (`self.Locations`) 2)
              (set `self.Locations` 0))))))
    (else
      (`SkeletalMeshComponent.PlayAnimation` (`self.Mesh`) "/Game/Characters/Mannequins/Animations/Manny/MM_Idle.MM_Idle" true))))

(event `MoveToRandomLocation`
  (bind _randomlocation (`NavigationSystemV1.K2_GetRandomLocationInNavigableRadius` (`self.K2_GetActorLocation`) 4000.0 null null))
  (`|AIMoveTo` self _randomlocation null
    (:`OnSuccess`
      (`self.MoveToRandomLocation`))))

(event `CanSprintAgain`
  (goto _label :!via `Reset`))

(event `self.BP_EnemyConception.OnTargetPerceptionUpdated`
  (params (Actor :type "Actor Object Reference") (Stimulus :type "AIStimulus Structure"))
  (cast `/Game/ThirdPerson/Blueprints/BP_ThirdPersonCharacter` Actor)
  (if (`self.CanSeePlayer`)
    (set `self.CanSeePlayer` false)
    (set `self.IsChasingPlayer` false)
    (`SkeletalMeshComponent.PlayAnimation` (`self.Mesh`) "/Game/Characters/Mannequins/Animations/Manny/MM_Walk_Fwd.MM_Walk_Fwd" true)
    (set `CharacterMovementComponent.MaxWalkSpeed` 150.0 (`self.CharacterMovement`))
    (`self.CanSprintAgain`)
    (`self.Patrol`)
    (else
      (set `self.CanSeePlayer` true))))

(event `self.ReceiveTick`
  (params (DeltaSeconds :type "Float (single-precision)"))
  (bind _alter_ui (`self.Alter_UI`))
  (if (`self.CanSeePlayer`)
    (set `self.Alertness` (+ (`self.Alertness`) 0.3))
    (else
      (set `self.Alertness` (+ (`self.Alertness`) -0.13))))
  (bind _aswidget_alert_icon (cast `/Game/Blueprints/Widget_Alert_Icon` (`WidgetComponent.GetWidget` (`self.Alter_UI`))))
  (`ProgressBar.SetPercent` (`/Game/Blueprints/Widget_Alert_Icon.Alert_Bar` _aswidget_alert_icon) (/ (`self.Alertness`) 100.0))
  (`SceneComponent.K2_SetWorldRotation` _alter_ui (`KismetMathLibrary.FindLookAtRotation` (`SceneComponent.K2_GetComponentLocation` _alter_ui) (`SceneComponent.K2_GetComponentLocation` (`PlayerCameraManager.TransformComponent` (`GameplayStatics.GetPlayerCameraManager` 0)))) false false)
  (if (>= (`self.Alertness`) 100.0)
    (`|ExecutionSequence`
      (:`then_0`
        (`/Engine/EditorBlueprintResources/StandardMacros.DoOnce` false :!label _label
          (:`Completed`
            (`SkeletalMeshComponent.PlayAnimation` (`self.Mesh`) "/Game/Characters/Mannequins/Animations/Quinn/MF_Run_Fwd.MF_Run_Fwd" true)
            (set `self.IsChasingPlayer` true)
            (set `CharacterMovementComponent.MaxWalkSpeed` 350.0 (`self.CharacterMovement`)))))
      (:`then_1`
        (`|AIMoveTo` self (0.0 0.0 0.0) (stale `self.BP_EnemyConception.OnTargetPerceptionUpdated` Actor))))))

(event `Killself`
  (`self.K2_DestroyActor`))

(fn `UserConstructionScript`)